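; Centaur enemy AI character that roams with looping AI MoveTo calls to random reachable points until it engages a player.
; PawnSensing sends it after heard noises or locks it onto "Hunter"-tagged pawns, and taking damage retargets it to the attacker.
; Attack mode repeatedly moves to the target's cardinal point, then routes a random attack through server-to-multicast events, applying delayed box-overlap damage.
; At zero health it stops, plays death montage and cry, then destroys itself.
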(event OnSeePawn(PawnSensing)
  (params (Pawn :type Pawn%20Object%20Reference))
  ;[0.15 0.15 0.15 0.5] Attack MultiCast
  (if (not (Variables|Default|GetDead?))
    (if (Actor|ActorHasTag Pawn "Hunter")
      (Utilities|FlowControl|Sequence
        (:then_0
          (Variables|Default|SetRoamTrue false)
          (Variables|Default|SetLockedInPawn Pawn)
          (CallFunction|AttackMode))
        (:then_1
          (Utilities|FlowControl|DoOnce false
            (:Completed
              (bind _spawnedsoundactor (Utilities|PlaySoundAttached "/Game/Core/SoundEffects/Kraken/SwitchModeCue.SwitchModeCue" 1.0))
              (bind _returnvalue (Animation|GetPlayLength _spawnedsoundactor))
              (Utilities|FlowControl|Delay _returnvalue)
              (Components|DestroyComponent _spawnedsoundactor))))))))

(event OnHearNoise(PawnSensing)
  (params (Instigator :type Pawn%20Object%20Reference) (Location :type Vector%20%28by%20ref%29 :default "0, 0, 0") (Volume :type Float%20%28single-precision%29))
  ;[0.15 0.15 0.15 0.5 50] Perform Attack
  (Variables|Default|SetRoamTrue false)
  (AI|AIMoveTo self Location Instigator 1.1e+02 false
    (:OnSuccess
      _)
    (:OnFail
      _))
  (Variables|Default|SetRoamTrue true)
  (CallFunction|Roam))

(event Custom|Roam
  (bind _charactermovement (Variables|Character|GetCharacterMovement))
  (bind _actorroam (Variables|Default|GetActorRoam))
  ;[0.15 0.15 0.15 0.5] Roam
  (if (Variables|Default|GetRoamTrue)
    (Utilities|FlowControl|Sequence
      (:then_0
        (AI|AIMoveTo self (.RandomLocation (AI|Navigation|GetRandomReachablePointinRadius (Transformation|GetActorLocation (select (Utilities|IsValid _actorroam) _actorroam self)) 1e+03 0 0)) 0 7e+01 false
          (:OnSuccess
            _)
          (:OnFail
            _))
        (if (Variables|Default|GetDead?)
          (Pawn|Components|CharacterMovement|DisableMovement _charactermovement)
          (Class|NavMovementInterface|StopActiveMovement _charactermovement)
          (Components|Movement|StopMovementImmediately _charactermovement)
          (else
            (Utilities|FlowControl|Delay 0.2)
            (CallFunction|Roam))))
      (:then_1
        (Utilities|FlowControl|DoOnce false :!label _label
          (:Completed
            (if (Utilities|IsValid (Variables|Default|GetAttackSound))
              (bind _spawnedsoundactor (Utilities|PlaySoundAttached "/Game/Core/SoundEffects/Kraken/RoamCue.RoamCue" 1.0 "/Game/Core/SoundEffects/Kraken/RoamCueAttenuation.RoamCueAttenuation"))
              (bind _output_get (Variables|Default|SetRoamSound _spawnedsoundactor))
              (bind _returnvalue (Animation|GetPlayLength _output_get))
              (Utilities|FlowControl|Delay _returnvalue)
              (goto _label Reset))))))))

(event Custom|AttackMulticast
  (bind _lockedinpawn (Variables|Default|GetLockedInPawn))
  ;[0.15 0.15 0.15 0.5 50] Perform Attack
  (Utilities|FlowControl|Sequence
    (:then_0
      (Effects|SpawnEmitteratLocation "/Game/StarterContent/Particles/P_Ambient_Dust.P_Ambient_Dust" (+ (Transformation|GetActorLocation) "0.000000,0.000000,10.000000"))
      (switch int (Math|Random|RandomIntegerinRange 0 3)
        (:0
          (Variables|Default|Setattackindex 0)
          (Variables|Default|SetAttack true)
          ;;[0.15 0.15 0.15 0.5] smash
          (Utilities|FlowControl|Delay 0.1)
          (Variables|Default|SetAttack false)
          (Utilities|FlowControl|Delay 0.5)
          (if (Collision|IsOverlappingActor (Variables|Default|GetBox) _lockedinpawn :!class /Script/Engine.PrimitiveComponent)
            (Game|Damage|ApplyDamage _lockedinpawn (Utilities|DamageRandom 0 0.7 1.0) 0 0)))
        (:1
          (Variables|Default|Setattackindex 1)
          (Variables|Default|SetAttack true)
          (Utilities|FlowControl|Delay 0.1)
          (Variables|Default|SetAttack false)
          (Utilities|FlowControl|Delay 0.5)
          (if (Collision|IsOverlappingActor (Variables|Default|GetBox) (Variables|Default|GetLockedInPawn) :!class /Script/Engine.PrimitiveComponent) :!label _label
            (Game|Damage|ApplyDamage (Variables|Default|GetLockedInPawn) (Utilities|DamageRandom 1 0.8 1.2) 0 0)))
        (:2
          (Variables|Default|Setattackindex 2)
          (Variables|Default|SetAttack true)
          (Utilities|FlowControl|Delay 0.1)
          (Variables|Default|SetAttack false)
          (Utilities|FlowControl|Delay 0.5)
          (goto _label))
        (:3
          (Variables|Default|Setattackindex 3)
          (Variables|Default|SetAttack true)
          (Utilities|FlowControl|Delay 0.1)
          (Variables|Default|SetAttack false)
          (Utilities|FlowControl|Delay 0.5)
          (if (Collision|IsOverlappingActor (Variables|Default|GetBox) (Variables|Default|GetLockedInPawn) :!class /Script/Engine.PrimitiveComponent)
            (Game|Damage|ApplyDamage (Variables|Default|GetLockedInPawn) (Utilities|DamageRandom 2 0.65 1.1) 0 0)))))
    (:then_1
      (if (Utilities|IsValid (Variables|Default|GetRoamSound))
        _))))

(event Custom|AttackOnServer
  ;[0.15 0.15 0.15 0.5 82] Attack Mode
  (CallFunction|AttackMulticast))

(event Custom|AttackMode
  (bind _charactermovement (Variables|Character|GetCharacterMovement))
  ;[0.15 0.15 0.15 0.5 82] Attack Mode
  (Variables|/Script/Engine.CharacterMovementComponent|SetMaxWalkSpeed (Variables|Character|GetCharacterMovement) (Variables|Default|GetMax%20Walk%20Speed))
  (Variables|Default|SetAttackModeSwitch true)
  (bind _asbp_third_person_character (Utilities|Casting|CastToBP_ThirdPersonCharacter (Variables|Default|GetLockedInPawn)))
  (bind _returnvalue (Default|GetCardinalPoint _asbp_third_person_character))
  (AI|AIMoveTo self (Transformation|GetWorldLocation _returnvalue) 0 1.1e+02 true
    (:OnSuccess
      (CallFunction|AttackonServer)
      (Utilities|FlowControl|Delay (Variables|Default|GetAttackRecoveryTime)))
    (:OnFail
      _))
  (if (Variables|Default|GetDead?)
    (Pawn|Components|CharacterMovement|DisableMovement _charactermovement)
    (Class|NavMovementInterface|StopActiveMovement _charactermovement)
    (Components|Movement|StopMovementImmediately _charactermovement)
    (else
      (CallFunction|AttackMode))))

(event EventBeginPlay
  ;[0.15 0 0 0.5 66] EventBeginPlay
  (Pawn|Components|CharacterMovement|SetMovementMode (Variables|Character|GetCharacterMovement) "MOVE_NavWalking" 0)
  (if (not (Variables|Default|GetDead?))
    (if (Variables|Default|GetRoamTrue)
      (CallFunction|Roam))))

(event Game|Damage|EventAnyDamage
  (params (Damage :type Float%20%28single-precision%29) (DamageType :type Damage%20Type%20Object%20Reference) (InstigatedBy :type Controller%20Object%20Reference) (DamageCauser :type Actor%20Object%20Reference))
  (bind _charactermovement (Variables|Character|GetCharacterMovement))
  ;[0.15 0.15 0.15 0.5 66] Event Any Damage
  (if (not (Variables|Default|GetDead?))
    (Variables|Default|SetHealth (Math|Float|Truncate (- (Variables|Default|GetHealth) Damage)))
    (Variables|Default|SetLockedInPawn (.AsBP%20Third%20Person%20Character (Utilities|Casting|CastToBP_ThirdPersonCharacter DamageCauser)))
    (CallFunction|AttackMode)
    (if (<= (Variables|Default|GetHealth) 0)
      (Utilities|FlowControl|DoOnce false
        (:Completed
          (Pawn|Components|CharacterMovement|DisableMovement _charactermovement)
          (Class|NavMovementInterface|StopActiveMovement _charactermovement)
          (Components|Movement|StopMovementImmediately _charactermovement)
          (Variables|Default|SetDead? true)
          (Animation|PlayAnimMontage "/Game/Kraken/Animations/KRAKEN_death_Montage.KRAKEN_death_Montage" 3.0 "None")
          ;;[0.15 0.15 0.15 0.5] Death Cye
          (Utilities|PlaySoundAttached "/Game/Core/SoundEffects/Kraken/DyingBeast.DyingBeast" 1.0)
          (Utilities|FlowControl|Delay 1e+01)
          (Actor|DestroyActor))))))

(fn ConstructionScript
  (Variables|/Script/Engine.CharacterMovementComponent|SetMaxWalkSpeed (Variables|Character|GetCharacterMovement) (/ (Variables|Default|GetMax%20Walk%20Speed) 1.5)))