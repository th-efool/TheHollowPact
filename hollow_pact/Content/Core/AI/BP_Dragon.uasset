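; Dragon boss AI that detects Hunter-tagged players by pawn sensing or sphere overlap, roars, then attacks.
; Distance picks walking or a one-time flight, using timelines for takeoff and trace-guided landing, velocity steering in the air.
; On the ground, AIMoveTo feeds random claw or fire montages, with box overlaps applying damage.
; Actions pass through server/multicast-named events driven by a mode enum; death unpossesses it, then reloads Valley_Demonstration after a delay.
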(event OnSeePawn(PawnSensing)
  (params (Pawn :type Pawn%20Object%20Reference))
  (bind _returnvalue (Transformation|GetActorLocation))
  (bind _returnvalue_2 (Transformation|GetActorLocation))
  (if (Variables|Default|GetDead?)
    ;[0.15 0.15 0.15 0.5 74] OnSenseMC
    (Components|DestroyComponent (Variables|Default|GetPawnSensing))
    (elif (Actor|ActorHasTag Pawn "Hunter")
      (Variables|Default|SetLockedInPawn Pawn)
      (Utilities|FlowControl|Sequence
        (:then_0
          (Utilities|FlowControl|DoOnce false
            (:Completed
              (Variables|Default|SetDoOnceRoar true)
              (bind _returnvalue_3 (Animation|PlayAnimMontage "/Game/QuadrapedCreatures/MountainDragon/Animations/Attack/ANIM_MOUNTAIN_DRAGON_spreadFire_Montage.ANIM_MOUNTAIN_DRAGON_spreadFire_Montage" 1.0 "None"))
              (if (Variables|Default|GetDead?)
                (Animation|StopAnimMontage "/Game/QuadrapedCreatures/MountainDragon/Animations/Attack/ANIM_MOUNTAIN_DRAGON_spreadFire_Montage.ANIM_MOUNTAIN_DRAGON_spreadFire_Montage")
                (else
                  (Utilities|FlowControl|Delay _returnvalue_3)
                  (Variables|Default|SetRoarDelayFinished true)
                  (if (> (Variables|Default|GetDragonPlayerDistance) (Variables|Default|GetMinFlightDistance))
                    (Development|PrintString "DEBUG TRUE")
                    (CallFunction|FlytoTPC)
                    (else
                      ;[0.15 0.15 0.15 0.5 114] GroundToAir
                      (Variables|Default|SetModesDragon "NewEnumerator3" :!label _label)
                      (CallFunction|WalktoTPC))))))))
        (:then_1
          (if (Variables|Default|GetRoarDelayFinished)
            (if (> (Variables|Default|GetDragonPlayerDistance) (Variables|Default|GetMinFlightDistance))
              ;[0.15 0 0 0.5 66] CODE PREVENTING  DRAGON FROM TAKING ON SECOND FLIGHT
              (if (Variables|Default|GetHasLandedOnce)
                (CallFunction|WalktoTPC)
                (elif (> (Variables|Default|GetDragonPlayerDistance) (Variables|Default|GetGlideDistance))
                  (Utilities|FlowControl|Sequence
                    (:then_0
                      (Variables|Default|SetModesDragon "NewEnumerator1")
                      (Utilities|FlowControl|Sequence
                        (:then_0
                          (Utilities|FlowControl|DoOnce false :!label _label_2
                            (:Completed
                              (if (not (Variables|Default|GetGroundToFlightAnimFinished))
                                (CallFunction|GroundtoGlideonServer)))))
                        (:then_1
                          (if (Variables|Default|GetGroundToFlightAnimFinished)
                            (CallFunction|FlytoTPC)))))
                    (:then_1
                      (goto _label_4 Reset)))
                  (else
                    (Utilities|FlowControl|Sequence
                      (:then_0
                        (Variables|Default|SetModesDragon "NewEnumerator2")
                        (Utilities|FlowControl|Sequence
                          (:then_0
                            (Utilities|FlowControl|DoOnce false :!label _label_3
                              (:Completed
                                (if (not (Variables|Default|GetGroundToFlightAnimFinished))
                                  (CallFunction|GroundtoFlyIpServer)))))
                          (:then_1
                            (if (Variables|Default|GetGroundToFlightAnimFinished)
                              (CallFunction|FlytoTPC)))))
                      (:then_1
                        (goto _label_4 Reset))))))
              (elif (Variables|Default|GetDoOnceRoar)
                (Utilities|FlowControl|Sequence
                  (:then_0
                    (Utilities|FlowControl|DoOnce true :!label _label_4
                      (:Completed
                        (CallFunction|LandonServer)
                        (Variables|Default|SetHasLandedOnce true)
                        (Variables|/Script/Engine.CharacterMovementComponent|SetbOrientRotationToMovement (Variables|Character|GetCharacterMovement) false)
                        (goto _label))))
                  (:then_1
                    (goto _label_2 Reset))
                  (:then_2
                    (goto _label_3 Reset))
                  (:then_3
                    (Utilities|FlowControl|DoOnce false) ; enters at Reset
                  )
                  (:then_4
                    (Utilities|FlowControl|DoOnce false) ; enters at Reset
                  ))
                (else
                  (goto _label))))))
        (:then_2
          (if (Utilities|Enum|Equal(Enum) (Variables|Default|GetModesDragon) "NewEnumerator3")
            (CallFunction|WalktoTPC)))))))

(event OnComponentBeginOverlap(Sphere)
  (params (OverlappedComponent :type Primitive%20Component%20Object%20Reference) (OtherActor :type Actor%20Object%20Reference) (OtherComp :type Primitive%20Component%20Object%20Reference) (OtherBodyIndex :type Integer) (bFromSweep :type Boolean) (SweepResult :type Hit%20Result%20Structure%20%28by%20ref%29))
  (bind _returnvalue (Transformation|GetActorLocation))
  (bind _returnvalue_2 (Transformation|GetActorLocation))
  (bind _returnvalue_3 (Components|GetOwner OverlappedComponent))
  ;[0.15 0.15 0.15 0.5 74] OnSenseMC
  (if (Actor|ActorHasTag _returnvalue_3 "Hunter")
    (bind _asbp_third_person_character (Utilities|Casting|CastToBP_ThirdPersonCharacter _returnvalue_3))
    (Variables|Default|SetLockedInPawn _asbp_third_person_character)
    (Utilities|FlowControl|Sequence
      (:then_0
        (Utilities|FlowControl|DoOnce false
          (:Completed
            (Variables|Default|SetDoOnceRoar true)
            (bind _returnvalue_4 (Animation|PlayAnimMontage "/Game/QuadrapedCreatures/MountainDragon/Animations/Attack/ANIM_MOUNTAIN_DRAGON_spreadFire_Montage.ANIM_MOUNTAIN_DRAGON_spreadFire_Montage" 1.0 "None"))
            (if (Variables|Default|GetDead?)
              (Animation|StopAnimMontage "/Game/QuadrapedCreatures/MountainDragon/Animations/Attack/ANIM_MOUNTAIN_DRAGON_spreadFire_Montage.ANIM_MOUNTAIN_DRAGON_spreadFire_Montage")
              (else
                (Utilities|FlowControl|Delay _returnvalue_4)
                (Variables|Default|SetRoarDelayFinished true)
                (if (> (Variables|Default|GetDragonPlayerDistance) (Variables|Default|GetMinFlightDistance))
                  (Development|PrintString "DEBUG TRUE")
                  (CallFunction|FlytoTPC)
                  (else
                    ;[0.15 0.15 0.15 0.5 114] GroundToAir
                    (Variables|Default|SetModesDragon "NewEnumerator3" :!label _label)
                    (CallFunction|WalktoTPC))))))))
      (:then_1
        (if (Variables|Default|GetRoarDelayFinished)
          (if (> (Variables|Default|GetDragonPlayerDistance) (Variables|Default|GetMinFlightDistance))
            ;[0.15 0 0 0.5 66] CODE PREVENTING  DRAGON FROM TAKING ON SECOND FLIGHT
            (if (Variables|Default|GetHasLandedOnce)
              (CallFunction|WalktoTPC)
              (elif (> (Variables|Default|GetDragonPlayerDistance) (Variables|Default|GetGlideDistance))
                (Utilities|FlowControl|Sequence
                  (:then_0
                    (Variables|Default|SetModesDragon "NewEnumerator1")
                    (Utilities|FlowControl|Sequence
                      (:then_0
                        (Utilities|FlowControl|DoOnce false :!label _label_2
                          (:Completed
                            (if (not (Variables|Default|GetGroundToFlightAnimFinished))
                              (CallFunction|GroundtoGlideonServer)))))
                      (:then_1
                        (if (Variables|Default|GetGroundToFlightAnimFinished)
                          (CallFunction|FlytoTPC)))))
                  (:then_1
                    (goto _label_4 Reset)))
                (else
                  (Utilities|FlowControl|Sequence
                    (:then_0
                      (Variables|Default|SetModesDragon "NewEnumerator2")
                      (Utilities|FlowControl|Sequence
                        (:then_0
                          (Utilities|FlowControl|DoOnce false :!label _label_3
                            (:Completed
                              (if (not (Variables|Default|GetGroundToFlightAnimFinished))
                                (CallFunction|GroundtoFlyIpServer)))))
                        (:then_1
                          (if (Variables|Default|GetGroundToFlightAnimFinished)
                            (CallFunction|FlytoTPC)))))
                    (:then_1
                      (goto _label_4 Reset))))))
            (elif (Variables|Default|GetDoOnceRoar)
              (Utilities|FlowControl|Sequence
                (:then_0
                  (Utilities|FlowControl|DoOnce true :!label _label_4
                    (:Completed
                      (CallFunction|LandonServer)
                      (Variables|Default|SetHasLandedOnce true)
                      (Variables|/Script/Engine.CharacterMovementComponent|SetbOrientRotationToMovement (Variables|Character|GetCharacterMovement) false)
                      (goto _label))))
                (:then_1
                  (goto _label_2 Reset))
                (:then_2
                  (goto _label_3 Reset))
                (:then_3
                  (Utilities|FlowControl|DoOnce false) ; enters at Reset
                )
                (:then_4
                  (Utilities|FlowControl|DoOnce false) ; enters at Reset
                ))
              (else
                (goto _label))))))
      (:then_2
        (if (Utilities|Enum|Equal(Enum) (Variables|Default|GetModesDragon) "NewEnumerator3")
          (CallFunction|WalktoTPC))))))

(event OnComponentBeginOverlap(Box)
  (params (OverlappedComponent :type Primitive%20Component%20Object%20Reference) (OtherActor :type Actor%20Object%20Reference) (OtherComp :type Primitive%20Component%20Object%20Reference) (OtherBodyIndex :type Integer) (bFromSweep :type Boolean) (SweepResult :type Hit%20Result%20Structure%20%28by%20ref%29))
  (if (Variables|Default|GetAagFeekRahaRukJao)
    (if (Actor|ActorHasTag OtherActor "Hunter")
      (Game|Damage|ApplyDamage OtherActor (Math|Random|RandomFloatinRange 4.0 12.0) 0 0))))

(event Custom|RoamOnServer
  ;[0.15 0.15 0.15 0.5 90] Roam On Server
  (CallFunction|RoamMulticast))

(event Custom|RoamMulticast
  ;[0.15 0.15 0.15 0.5 90] Roam On Server
  (if (Utilities|Enum|Equal(Enum) (Variables|Default|GetModesDragon) "NewEnumerator6")
    (AI|AIMoveTo self (.RandomLocation (AI|Navigation|GetRandomReachablePointinRadius (Transformation|GetActorLocation) 1e+03 0 0)) 0 7e+01 false
      (:OnSuccess
        _)
      (:OnFail
        _))
    (if (Variables|Default|GetDead?)
      (CallFunction|DeathonServer)
      (else
        (Utilities|FlowControl|Delay 5.0)
        (CallFunction|RoamonServer)))))

(event Custom|GroundToGlideOnServer
  ;[0.15 0.15 0.15 0.5 114] GroundToAir
  (CallFunction|GroundtoGlide))

(event Custom|LandOnServer
  ;[0.15 0.15 0.15 0.5 42] Land On Server
  (CallFunction|LandonServerMulticast))

(event Custom|LandOnServerMulticast
  ;[0.15 0.15 0.15 0.5 42] Land On Server
  (if (Variables|Default|GetDead?)
    (CallFunction|DeathonServer)
    (else
      (Pawn|Components|CharacterMovement|SetMovementMode (Variables|Character|GetCharacterMovement) "MOVE_Walking" 0)
      (Variables|Default|SetGroundToFlightAnimFinished false)
      (Variables|Default|SetBroHasLanded true)
      (CallFunction|ZaaminHainKaha)
      (if (> (Math|Vector|VectorLength (Transformation|GetVelocity)) 1e+01)
        (Animation|PlayAnimMontage "/Game/QuadrapedCreatures/MountainDragon/Animations/Workspace/ANIM_MOUNTAIN_DRAGON_glidePosToLanding_Montage.ANIM_MOUNTAIN_DRAGON_glidePosToLanding_Montage" 1.0 "None")
        (Variables|Default|SetModesDragon "NewEnumerator3")
        (bind _newtrack_0 (Timeline|SlurpForLerp PlayFromStart)
          (:Update
            (Variables|Default|SetIsInProcessOfLanding true)
            (Transformation|SetActorRelativeLocation (Math|Vector|Lerp(Vector) (Transformation|GetActorLocation) (Variables|Default|GetTheHillDieOn) _newtrack_0) true))
          (:Finished
            (Variables|Default|SetIsInProcessOfLanding false)
            (CallFunction|WalktoTPC)))
        (else
          (Animation|PlayAnimMontage "/Game/QuadrapedCreatures/MountainDragon/Animations/Workspace/ANIM_MOUNTAIN_DRAGON_FlyStationaryToLanding_Montage.ANIM_MOUNTAIN_DRAGON_FlyStationaryToLanding_Montage" 1.0 "None")
          (Variables|Default|SetModesDragon "NewEnumerator3")
          (Timeline|SlurpForLerp PlayFromStart))))))

(event Custom|DeathOnServer
  ;[0.15 0.15 0.15 0.5 74] DeathOnServer
  (CallFunction|DeathMulticast))

(event Custom|FlyToTPCMultiCast
  (bind _lockedinpawn (Variables|Default|GetLockedInPawn))
  (bind _returnvalue (Transformation|GetActorLocation _lockedinpawn))
  ;[0.15 0.15 0.15 0.5 50] Fly To Player Character
  (if (Variables|Default|GetDead?)
    (CallFunction|DeathonServer)
    (elif (< (Variables|Default|GetDragonPlayerDistance) (Variables|Default|GetMinLandDistance))
      (Variables|/Script/Engine.MovementComponent|SetVelocity (Variables|Character|GetCharacterMovement) "0, 0, 0")
      (else
        (Variables|/Script/Engine.MovementComponent|SetVelocity (Variables|Character|GetCharacterMovement) (* (Math|Vector|GetUnitDirection(Vector) (Transformation|GetActorLocation) (Math|Vector|MakeVector (.x _returnvalue) (.y _returnvalue) (.z (Transformation|GetActorLocation)))) (Math|Conversions|ToVector(Float) (Variables|Default|GetDragonFlySpeed))))))))

(event Custom|FlyToTPC
  ;[0.15 0.15 0.15 0.5 50] Fly To Player Character
  (CallFunction|FlytoTPCMultiCast))

(event Custom|WalkToTPC
  ;[0.15 0.06562 0.06562 0.5 98] WAlk To Player Character
  (CallFunction|WalktoTPCMulti))

(event Custom|WalkToTPCMulti
  (if (Variables|Default|GetDead?)
    (CallFunction|DeathonServer)
    (elif (not (Variables|Default|GetIsInProcessOfLanding))
      (if (Utilities|Enum|Equal(Enum) (Variables|Default|GetModesDragon) "NewEnumerator3")
        ;[0.15 0.06562 0.06562 0.5 98] WAlk To Player Character
        (if (Variables|Default|GetAagFeekRahaRukJao)
          (AI|AIMoveTo self "0, 0, 0" (Variables|Default|GetLockedInPawn) 5e+02 true
            (:then
              (if (Variables|Default|GetDead?)
                (CallFunction|DeathonServer :!label _label)))
            (:OnSuccess
              (if (Variables|Default|GetDead?)
                (goto _label)
                (else
                  (switch int (Math|Random|RandomIntegerinRange 0 3)
                    (:0
                      (bind _returnvalue (Animation|PlayAnimMontage "/Game/QuadrapedCreatures/MountainDragon/Animations/Attack/ATTACK_LeftClawsAttackMontage.ATTACK_LeftClawsAttackMontage" 1.0 "None"))
                      (Variables|Default|SetAagFeekRahaRukJao false)
                      (Utilities|FlowControl|Delay (* _returnvalue 1.4)))
                    (:1
                      (bind _returnvalue_2 (Animation|PlayAnimMontage "/Game/QuadrapedCreatures/MountainDragon/Animations/Attack_ClawsAttack2HitComboForward_Montage.Attack_ClawsAttack2HitComboForward_Montage" 1.0 "None"))
                      (Variables|Default|SetAagFeekRahaRukJao false)
                      (Utilities|FlowControl|Delay (* _returnvalue_2 1.6)))
                    (:2
                      (bind _returnvalue_3 (Animation|PlayAnimMontage "/Game/QuadrapedCreatures/MountainDragon/Animations/Attack/ATTACK_RightClawsAttackMontage.ATTACK_RightClawsAttackMontage" 1.0 "None"))
                      (Variables|Default|SetAagFeekRahaRukJao false)
                      (Utilities|FlowControl|Delay (* _returnvalue_3 1.4)))
                    (:3
                      (bind _returnvalue_4 (Animation|PlayAnimMontage "/Game/QuadrapedCreatures/MountainDragon/Animations/Attack/ANIM_MOUNTAIN_DRAGON_spreadFire_Montage.ANIM_MOUNTAIN_DRAGON_spreadFire_Montage" 1.0 "None"))
                      (Variables|Default|SetAagFeekRahaRukJao false)
                      (Utilities|FlowControl|Delay (* _returnvalue_4 1.2))))
                  (Variables|Default|SetAagFeekRahaRukJao true)
                  (CallFunction|WalktoTPC))))))))))

(event Custom|DeathMulticast
  (Pawn|Components|CharacterMovement|SetMovementMode (Variables|Character|GetCharacterMovement) "MOVE_Walking" 0)
  (Utilities|FlowControl|Sequence
    (:then_0
      (Development|PrintString "Hello Darkness My Old Friend" true true "(R=0.845083,G=1.000000,B=0.590425,A=1.000000)"))
    (:then_1
      ;[0.15 0.15 0.15 0.5] Stop All Anim Montages
      (Utilities|FlowControl|Sequence
        (:then_0
          (if (Variables|Default|GetDoOnceRoar)
            (if (not (Variables|Default|GetGroundToFlightAnimFinished))
              (Animation|StopAnimMontage "/Game/QuadrapedCreatures/MountainDragon/Animations/Attack/ANIM_MOUNTAIN_DRAGON_spreadFire_Montage.ANIM_MOUNTAIN_DRAGON_spreadFire_Montage"))))
        (:then_1
          (if (Variables|Default|GetDeathProtectAnimMontage1)
            (if (not (Variables|Default|GetGroundToFlightAnimFinished))
              (Animation|StopAnimMontage "/Game/QuadrapedCreatures/MountainDragon/Animations/DoneWork/NoRM_TakeOffToGlide.NoRM_TakeOffToGlide"))))
        (:then_2
          (if (Variables|Default|GetDeathProtectAnimMontage2)
            (if (not (Variables|Default|GetGroundToFlightAnimFinished))
              (Animation|StopAnimMontage "/Game/QuadrapedCreatures/MountainDragon/Animations/DoneWork/NoRMFuckedUpTakeoffStationary.NoRMFuckedUpTakeoffStationary"))))))
    (:then_2
      (Utilities|FlowControl|DoOnce false
        (:Completed
          (Pawn|UnPossess (Pawn|GetController)))))))

(event Custom|GroundToGlide
  (bind _returnvalue (Transformation|GetActorLocation))
  ;[0.15 0.15 0.15 0.5 114] GroundToAir
  (Utilities|FlowControl|DoOnce false
    (:Completed
      (Variables|Default|SetDeathProtectAnimMontage2 true)
      (Variables|Default|SetModesDragon "NewEnumerator1")
      (Variables|Default|SetFlying true)
      (Pawn|Components|CharacterMovement|SetMovementMode (Variables|Character|GetCharacterMovement) "MOVE_Flying" 0)
      (bind _returnvalue_2 (Animation|PlayAnimMontage "/Game/QuadrapedCreatures/MountainDragon/Animations/DoneWork/NoRM_TakeOffToGlide.NoRM_TakeOffToGlide" 1.0 "None"))
      (Utilities|FlowControl|Sequence
        (:then_0
          (Utilities|FlowControl|Delay 0.1)
          (bind _newtrack_0 (Timeline|LandToGlide PlayFromStart)
            (:Update
              (Transformation|SetActorRelativeLocation (Math|Vector|MakeVector (.x _returnvalue) (.y _returnvalue) _newtrack_0) true)
              (if (Variables|Default|GetDead?)
                (Animation|StopAnimMontage "/Game/QuadrapedCreatures/MountainDragon/Animations/DoneWork/NoRM_TakeOffToGlide.NoRM_TakeOffToGlide")
                (else
                  (CallFunction|SmoothlyLookatPlayeronServer))))
            (:Finished
              (CallFunction|FlytoTPC))))
        (:then_1
          (Utilities|FlowControl|Delay _returnvalue_2)
          (Variables|Default|SetGroundToFlightAnimFinished true))))))

(event Custom|SmoothlyLookAtPlayerMulti
  ;[0.15 0.15 0.15 0.5 82] SmoothlyLookAtPlayerOnSErver
  (Transformation|SetActorRotation (Math|Rotator|MakeRotator 0.0 0.0 (.yaw (Math|Rotator|Lerp(Rotator) (Transformation|GetActorRotation) (Math|Rotator|FindLookatRotation (Transformation|GetActorLocation) (Transformation|GetActorLocation (Variables|Default|GetLockedInPawn))) 0.2)))))

(event Custom|GroundToFlyIP
  (bind _returnvalue (Transformation|GetActorLocation))
  (Variables|/Script/Engine.CharacterMovementComponent|SetbOrientRotationToMovement (Variables|Character|GetCharacterMovement) true)
  ;[0.15 0.15 0.15 0.5 114] GroundToAir
  (Utilities|FlowControl|DoOnce false
    (:Completed
      (Variables|Default|SetModesDragon "NewEnumerator2")
      (Variables|Default|SetDeathProtectAnimMontage1 true)
      (Variables|Default|SetFlying true)
      (Pawn|Components|CharacterMovement|SetMovementMode (Variables|Character|GetCharacterMovement) "MOVE_Flying" 0)
      (bind _returnvalue_2 (Animation|PlayAnimMontage "/Game/QuadrapedCreatures/MountainDragon/Animations/DoneWork/NoRMFuckedUpTakeoffStationary.NoRMFuckedUpTakeoffStationary" 0.6 "None"))
      (Utilities|FlowControl|Sequence
        (:then_0
          (Utilities|FlowControl|Delay 0.1)
          (bind _newtrack_0 (Timeline|FlyBaby PlayFromStart)
            (:Update
              (Transformation|SetActorRelativeLocation (Math|Vector|MakeVector (.x _returnvalue) (.y _returnvalue) (+ _newtrack_0 31.0)) true)
              (if (Variables|Default|GetDead?)
                (Animation|StopAnimMontage "/Game/QuadrapedCreatures/MountainDragon/Animations/DoneWork/NoRMFuckedUpTakeoffStationary.NoRMFuckedUpTakeoffStationary")
                (else
                  (CallFunction|SmoothlyLookatPlayeronServer))))
            (:Finished
              (CallFunction|FlytoTPC))))
        (:then_1
          (Utilities|FlowControl|Delay _returnvalue_2)
          (Variables|Default|SetGroundToFlightAnimFinished true))))))

(event Custom|SmoothlyLookAtPlayerOnServer
  ;[0.15 0.15 0.15 0.5 82] SmoothlyLookAtPlayerOnSErver
  (CallFunction|SmoothlyLookatPlayerMulti))

(event Custom|ZaaminHainKaha
  (bind (_outhit _returnvalue) (Collision|LineTraceByChannel (Transformation|GetWorldLocation (Variables|Default|GetArrow1)) (+ (Transformation|GetWorldLocation (Variables|Default|GetArrow1)) "0.000000,0.000000,-10000.000000") "TraceTypeQuery1" false 0 "None"))
  (if _returnvalue
    (Variables|Default|SetTheHillDieOn (.location _outhit))))

(event Custom|GroundToFlyIpServer
  ;[0.15 0.15 0.15 0.5 114] GroundToAir
  (CallFunction|GroundtoFlyIP))

(event EventBeginPlay
  ;[0.15 0.15 0.15 0.5 98] Event Begin Play
)

(event EventTick
  (params (DeltaSeconds :type Float%20%28single-precision%29))
  (bind _returnvalue (Transformation|GetActorTransform))
  (bind _lockedinpawn (Variables|Default|GetLockedInPawn))
  (bind _returnvalue_2 (Transformation|GetActorLocation _lockedinpawn))
  (bind _returnvalue_3 (Math|Rotator|FindRelativeLookatRotation _returnvalue _returnvalue_2))
  ;[0.15 0.15 0.15 0.5 90] EVENT TICK (1) YAW PITCH (2)PlayerDistance (3)LookAtPlayer
  (if (not (Variables|Default|GetDead?))
    (Utilities|IsValid _lockedinpawn
      (:Is%20Valid
        (Utilities|FlowControl|Sequence
          (:then_0
            (Variables|Default|SetYaw (.yaw _returnvalue_3))
            (Variables|Default|SetPitch (.pitch _returnvalue_3)))
          (:then_1
            (bind _output_get (Variables|Default|SetDragonPlayerDistance (Math|Float|Absolute(Float) (Math|Vector|VectorLength (- (Transformation|GetActorLocation (Variables|Default|GetLockedInPawn)) (Transformation|GetActorLocation))))))
            (Development|PrintString (Utilities|String|ToString(Float) _output_get)))
          (:then_2
            (if (or (Utilities|Enum|NotEqual(Enum) (Variables|Default|GetModesDragon) "NewEnumerator5") (Utilities|Enum|NotEqual(Enum) (Variables|Default|GetModesDragon) "NewEnumerator6"))
              (if (Variables|Default|GetRoarDelayFinished)
                (if (Variables|Default|GetGroundToFlightAnimFinished)
                  (CallFunction|SmoothlyLookatPlayeronServer)))))
          (:then_3))))))

(event Game|Damage|EventAnyDamage
  (params (Damage :type Float%20%28single-precision%29) (DamageType :type Damage%20Type%20Object%20Reference) (InstigatedBy :type Controller%20Object%20Reference) (DamageCauser :type Actor%20Object%20Reference))
  ;[0.15 0.08516 0.08516 0.5 58] Event Take Damage
  (Variables|Default|SetHealth (Math|Float|Truncate (- (Variables|Default|GetHealth) Damage)))
  (Utilities|FlowControl|Sequence
    (:then_0
      ;;[0.15 0.15 0.15 0.5] AI MOVE TO PLAYER
      ;; if it hasn't taken flight then it does
      (Utilities|IsValid (Variables|Default|GetLockedInPawn)
        (:Is%20Not%20Valid
          (if (Actor|ActorHasTag DamageCauser "Hunter")
            _))))
    (:then_1
      (if (<= (Variables|Default|GetHealth) 0)
        (Utilities|FlowControl|DoOnce false
          (:Completed
            (Variables|Default|SetDead? true)
            (CallFunction|DeathMulticast)
            (Utilities|FlowControl|Delay 1e+01)
            (Game|OpenLevel(byObjectReference) "/Game/Valley_Gul/Maps/Valley_Demonstration.Valley_Demonstration")))))))

(fn ConstructionScript
  (Components|Sphere|SetSphereRadius (Variables|Default|GetSphere) (Variables|Default|GetIn%20Sphere%20Radius) true))

(fn OnRepCombat)

(fn OnRepModesDragon)

(fn OnRepHealth)