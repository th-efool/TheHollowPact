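; Weapon pickup actor that hands its weapon to the character who interacts with it.
; On interact it plays a clank and passes its weapon index, itself and its transform to the character's AddWeaponToHandOnServer.
; The index also selects a pickup sound: positional rifle, sniper or grenade launcher ammo sounds, or a 2D bow sound.
; DestroyMePublically forwards to a multicast-named event that destroys the actor, but nothing active here calls it.
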(event Custom|DestroyMePublically
  (CallFunction|DestroyMePublicallyMulticastIT))

(event Custom|DestroyMePublicallyMulticastIT
  (Actor|DestroyActor))

(event EventBeginPlay)

(event Collision|EventActorBeginOverlap
  (params (OtherActor :type Actor%20Object%20Reference)))

(event EventTick
  (params (DeltaSeconds :type Float%20%28single-precision%29)))

(event EventInteractPitchFork
  (params (CharacterPickingUp :type BP%20Third%20Person%20Character%20Object%20Reference))
  (bind _weapontospawninhandindex (Variables|Default|GetWeaponToSpawnInHandIndex))
  (Audio|PlaySoundatLocation "/Game/Core/SoundEffects/clank2.clank2" (Transformation|GetActorLocation) "0, 0, 0" 1.0 1.0 0.0 0 0 0 0)
  (Default|AddWeapontoHandonServer CharacterPickingUp _weapontospawninhandindex self (Transformation|GetActorTransform))
  (switch int _weapontospawninhandindex
    (:1
      (Audio|PlaySoundatLocation "/Game/StarterContent/Military/MilitaryWeapSilver/Sound/Rifle/Wavs/Rifle_AmmoPickup.Rifle_AmmoPickup" (Transformation|GetActorLocation) "0, 0, 0" 1.0 1.0 0.0 0 0 0 0 :!label _label))
    (:2
      (Audio|PlaySoundatLocation "/Game/StarterContent/Military/MilitaryWeapSilver/Sound/SniperRifle/Wavs/SniperRifle_AmmoPickup.SniperRifle_AmmoPickup" (Transformation|GetActorLocation) "0, 0, 0" 1.0 1.0 0.0 0 0 0 0 :!label _label_2))
    (:3
      (Audio|PlaySoundatLocation "/Game/StarterContent/Military/MilitaryWeapSilver/Sound/GrenadeLauncher/Wavs/GrenadeLauncher_AmmoPickup.GrenadeLauncher_AmmoPickup" (Transformation|GetActorLocation) "0, 0, 0" 1.0 1.0 0.0 0 0 0 0 :!label _label_3))
    (:4
      (goto _label))
    (:5
      (goto _label_2))
    (:6
      (goto _label_3))
    (:7
      (Audio|PlaySound2D "/Game/Core/SoundEffects/DeveloperBowPickedSound.DeveloperBowPickedSound" 1.0 1.0 0.0 0 0 :!label _label_4))
    (:8
      (goto _label_4))))

(fn ConstructionScript
  (|CallParentFunction))