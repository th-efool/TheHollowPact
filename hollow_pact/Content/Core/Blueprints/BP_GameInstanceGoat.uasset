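; Game instance that handles menus, session hosting and joining, and the solo How To Play launch.
; Multiplayer events create a four-player session with a toggleable LAN flag or join a search result; hosting success opens MasterMeLevel without the listen option.
; How To Play sets solo and tutorial-screen flags before opening that level.
; Menu functions display widgets, but the main menu's validity check reads a different variable than it assigns.
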(event Custom|ControlMenuShow)

(event Custom|Start_HowToPlay
  (Variables|Default|SetIsSoloMode? true)
  (Variables|Default|SetHowToPlayScreen true)
  (Game|OpenLevel(byObjectReference) "/Game/Core/MenuMaps/MasterMeLevel.MasterMeLevel"))

(event Custom|CreateMultiplayerSession
  (Variables|Default|SetIsSoloMode? false)
  (|Session (Game|GetPlayerController 0) 4 (Variables|Default|GetIsLanConnectino?) true
    (:OnSuccess
      (Game|OpenLevel(byObjectReference) "/Game/Core/MenuMaps/MasterMeLevel.MasterMeLevel"))
    (:OnFailure
      (Development|PrintString "Failed to create a session -- game instance --create session"))))

(event Custom|JoinMultiplayerSession
  (params (Search%20Result :type Blueprint%20Session%20Result%20Structure))
  (Variables|Default|SetIsSoloMode? false)
  (|JoinSession (Game|GetPlayerController 0) Search%20Result
    (:OnFailure
      (Development|PrintString "Failed to join a session -- game instance --JoinMultiplayerSession"))))

(fn UIGameShowMainMenu
  (bind _returnvalue (Game|GetPlayerController 0))
  (Utilities|IsValid (Variables|Default|GetWB_MainMenu)
    (:Is%20Valid
      _)
    (:Is%20Not%20Valid
      (bind _returnvalue_2 (UserInterface|CreateWidget "/Game/Core/Widgets/W_MainMenuP.W_MainMenuP_C" _returnvalue))
      (bind _output_get (Variables|Default|SetMainMenuTest _returnvalue_2))))
  (UserInterface|Viewport|AddtoViewport _output_get 0)
  (Input|SetInputModeUIOnly _returnvalue 0 "DoNotLock" false)
  (Variables|/Script/Engine.PlayerController|SetbShowMouseCursor _returnvalue true)
  (return))

(fn UIShowMultiplayerMenu
  (Utilities|IsValid (Variables|Default|GetMultiplayer%20Menu)
    (:Is%20Valid
      _)
    (:Is%20Not%20Valid
      (bind _returnvalue (UserInterface|CreateWidget "/Game/Core/Widgets/W_MultiplayerMenu.W_MultiplayerMenu_C" (Game|GetPlayerController 0)))
      (bind _output_get (Variables|Default|SetMultiplayer%20Menu _returnvalue))))
  (UserInterface|Viewport|AddtoViewport _output_get 0)
  (return))

(fn ChangeConnectionType
  (if (Variables|Default|GetIsLanConnectino?)
    (Variables|Default|SetIsLanConnectino? false)
    (else
      (Variables|Default|SetIsLanConnectino? true)))
  (return (Variables|Default|GetIsLanConnectino?)))