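; Game mode for a Prop Hunt match, running the lobby, prop selection, match timer and restart.
; Logins fill a player list and, from two players before the game starts, set a lobby timer that picks a random player to possess a newly spawned prop character.
; Players receive role and countdown widgets, and timer expiry gives the prop the win.
; Ending the match shows win screens, then reloads through ServerTravel.
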(event Custom|StartGameLobbyTimer
  ;[0.15 0.15 0.15 0.5] SettingUp Players In Lobby
  ;;[0.15 0.15 0.15 0.5] Lobby Timer
  (Utilities|Time|SetTimerbyEvent (delegate Custom|ChoosePropCharacter) 3e+01))

(event Custom|ChoosePropCharacter
  (bind _players (Variables|Default|GetPlayers))
  ;[0.15 0.15 0.15 0.5] SettingUp Players In Lobby
  (Variables|Default|SetHasGameStarted? true)
  (bind _output_get (Variables|Default|SetThePropHuntPlayer (Utilities|Array|Get(acopy) _players (Math|Random|RandomIntegerinRange 0 (Utilities|Array|Length _players)))))
  (Utilities|IsValid _output_get
    (:Is%20Valid
      (bind _returnvalue (Game|SpawnActorfromClass "/Game/Core/Blueprints/BP_Prop_Character.BP_Prop_Character_C" (Math|Transform|MakeTransform (Variables|Default|GetPropStartLocation) "0, 0, 0" "1.000000,1.000000,1.000000") "Undefined" "MultiplyWithRoot" 0 0))
      (CameraShake|StopAllCameraShakes (Variables|/Script/Engine.PlayerController|GetPlayerCameraManager (Variables|Default|GetThePropHuntPlayer)) true)
      (Actor|DestroyActor (Pawn|GetControlledPawn (Variables|Default|GetThePropHuntPlayer)))
      (Utilities|FlowControl|Delay 0.3)
      (Pawn|Possess (Variables|Default|GetThePropHuntPlayer) _returnvalue)
      (Utilities|FlowControl|Sequence
        (:then_0
          ;[0.15 0.15 0.15 0.5] SettingUpWidgets
          (Class|BPIPropHuntController|SetUpPropWidget(Message) (Variables|Default|GetThePropHuntPlayer) true)
          (for _array_element (Variables|Default|GetPlayers)
            (Utilities|IsValid _array_element
              (:Is%20Valid
                ;[0.15 0.15 0.15 0.5] Initiate Widget/Setting on EAHC PLAYER or HIS HUD
                (Utilities|FlowControl|Sequence
                  (:then_0
                    (bind _theprophuntplayer (Variables|Default|GetThePropHuntPlayer)
                      (:then
                        (if (!= _theprophuntplayer _array_element)
                          (Class|BPIPropHuntController|SetUpPropWidget(Message) _array_element false)))
                      (:else)))
                  (:then_1
                    (Class|BPIPropHuntController|SetMatchLengthandBeginCountdown(Message) _array_element (Variables|Default|GetMatchLength)))))))
          (CallFunction|StartGameLoopTimer))
        (:then_1
          (for (_array_element_2 _array_index) (Variables|Default|GetPlayers)
            (Input|EnableInput (Game|GetPlayerCharacter _array_index) _array_element_2)))))
    (:Is%20Not%20Valid
      (Utilities|FlowControl|Delay 1.0)
      (CallFunction|ChoosePropCharacter))))

(event Custom|StartGameLoopTimer
  ;[0.15 0.15 0.15 0.5 65] GameLoop Timer
  (bind _returnvalue (Utilities|Time|SetTimerbyEvent (delegate Custom|EndGame) (Variables|Default|GetMatchLength)))
  (Variables|Default|SetGameLoopTimer _returnvalue))

(event Custom|EndGame
  ;[0.15 0.15 0.15 0.5 65] GameLoop Timer
  ;[0.15 0.15 0.15 0.5] End Game Widgets Update
  (CallFunction|EndtheGame true))

(event Custom|StartNewGame
  (Development|ExecuteConsoleCommand "ServerTravel MasterMeLevel" 0))

(event EventEndtheGame
  (params (PropWon :type Boolean))
  ;[0.15 0.15 0.15 0.5] End Game Widgets Update
  (Utilities|Time|ClearandInvalidateTimerbyHandle (Variables|Default|GetGameLoopTimer))
  (bind _output_get (Variables|Default|SetProp%20Won PropWon))
  (for _array_element (Variables|Default|GetPlayers)
    (Utilities|IsValid _array_element
      (:Is%20Valid
        (Class|BPIPropHuntController|ShowWinScreenWIdget(Message) _array_element _output_get))))
  (Utilities|Time|SetTimerbyEvent (delegate Custom|StartNewGame) 4.0))

(event EventPostLogin
  (params (NewPlayer :type Player%20Controller%20Object%20Reference))
  ;[0.15 0.15 0.15 0.5] SettingUp Players In Lobby
  (Utilities|Array|Add (Variables|Default|GetPlayers) NewPlayer)
  (if (not (Variables|Default|GetHasGameStarted?))
    (if (>= (Utilities|Array|Length (Variables|Default|GetPlayers)) 2)
      ;;[0.15 0.15 0.15 0.5] Lobby Timer
      (CallFunction|StartGameLobbyTimer))))

(fn ConstructionScript)