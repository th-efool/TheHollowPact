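; Player controller for a Prop Hunt game that creates the local player's main HUD and acts as the bridge for updating it.
; Public events mostly forward to client-named events that drive the widget: prop setup, health, ammo, explosives, minimap, popups, match countdown and win screen.
; Crosshair events handle visibility, hit animation and spread mapped from velocity passed in, since the controller holds the HUD reference.
; Compass widget creation is present but disconnected.
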(event Custom|SetPropOnClient
  (params (IsProp :type Boolean))
  ;[0.15 0.15 0.15 0.5] SetUp Widget Screen
  (Default|HUDSetUpPropWidgets (Variables|Default|GetW_MainHudReference) IsProp))

(event Custom|Crosshair%20Hide%20OwningClient
  (params (isCombat :type Boolean))
  (bind _w_mainhudreference (Variables|Default|GetW_MainHudReference))
  ;[0.15 0.15 0.15 0.5] Combat State Update
  ;;[0.15 0.15 0.15 0.5] Crosshair Visibilty Update
  (if isCombat
    (Default|UpdateCrosshairVisibility _w_mainhudreference "Visible")
    (else
      (Default|UpdateCrosshairVisibility _w_mainhudreference "Hidden"))))

(event Custom|HUDUpdateLandMines
  (params (Number :type Integer))
  (Default|UpdateLandMineNumber (Variables|Default|GetW_MainHudReference) Number))

(event Custom|HUDUpdateGrenades
  (params (Number :type Integer))
  (Class|BPIPropHuntController|UpdateGrenades(Message) (Variables|Default|GetW_MainHudReference) Number))

(event Custom|HUDPlayMessagePopUp
  (params (MessagePopUp :type Text))
  (bind _w_mainhudreference (Variables|Default|GetW_MainHudReference))
  (Utilities|IsValid _w_mainhudreference
    (:Is%20Valid
      (Default|PlayMessagePopUp _w_mainhudreference MessagePopUp))))

(event Custom|Setup%20Crosshair%20Spread%20on%20Client
  (params (Velocity :type Vector))
  ;[0.15 0.15 0.15 0.5] CrosshairSpread (the reason why we made it here, cuz our CONTROLLER HAS REFERENCE to HUD not OUR CHARACTER, however from our character we do need to COMMUNICATE VELOCITY
  (Variables|/Game/Core/Widgets/W_MainHud.W_MainHud_C|SetCrosshairSpread (Variables|Default|GetW_MainHudReference) (Math|Float|MapRangeClamped (Math|Vector|VectorLength Velocity) 0.0 4e+02 5.0 7e+01)))

(event Custom|Update%20Health%20On%20Client
  (params (Health :type Integer))
  ;[0.15 0.15 0.15 0.5] Health Update
  (Default|UpdateHealthBar (Variables|Default|GetW_MainHudReference) Health))

(event Custom|ShowWinScreenOnClient
  (params (PropWon? :type Boolean) (AreWeTheProp? :type Boolean))
  ;[0.15 0.15 0.15 0.5] WinScreenWidget
  (Default|ShowWinScreen (Variables|Default|GetW_MainHudReference) PropWon? AreWeTheProp?))

(event Custom|HudUpdateGunHandAmmoMag
  (params (HunIndexInHand :type Integer) (MagzineAmmo :type Integer) (InventoryAmmo :type Integer))
  (Default|UpdateGunIndexGunMagzineInventoryFC (Variables|Default|GetW_MainHudReference) HunIndexInHand MagzineAmmo InventoryAmmo))

(event Custom|SetmatchLengthOnClient
  (params (Time :type Float%20%28double-precision%29))
  (bind _w_mainhudreference (Variables|Default|GetW_MainHudReference))
  ;[0.15 0.15 0.15 0.5] Set 1)GameTimeLength 2)Trigger the Start Countdown
  (Development|PrintText (Utilities|Text|ToText(Float) Time "HalfToEven"))
  (Default|SetMatchLength _w_mainhudreference Time)
  (Default|StartTimer _w_mainhudreference))

(event Custom|ShowCrosshaiirHitOnClient
  ;[0.15 0.15 0.15 0.5] CrossHair Hit
  (Default|PlayHitAnimation (Variables|Default|GetW_MainHudReference)))

(event Custom|HudUpdateAmmoMag
  (params (Mag :type Integer) (Inventory :type Integer))
  (Default|UpdateGunMagzineInventoryFC (Variables|Default|GetW_MainHudReference) Mag Inventory))

(event Custom|UpdateMiniMapOnOwningClient
  (params (Reference%20to%20Material%20Mini%20Map :type Material%20Interface%20Object%20Reference))
  (Default|MiniMaptoClientSet (Variables|Default|GetW_MainHudReference) Reference%20to%20Material%20Mini%20Map))

(event EventBeginPlay
  (bind _self self)
  ;[0.15 0.15 0.15 0.5] Creating Widgets For Clients
  (Utilities|FlowControl|Sequence
    (:then_0
      (if (Pawn|IsLocalPlayerController)
        (Input|SetInputModeGameOnly _self false)
        (Variables|Default|SetbShowMouseCursor _self false)))
    (:then_1
      (Networking|SwitchHasAuthority
        (:Authority
          (if (Pawn|IsLocalPlayerController)
            (bind _returnvalue (UserInterface|CreateWidget "/Game/Core/Widgets/W_MainHud.W_MainHud_C" self :!label _label))
            (bind _output_get (Variables|Default|SetW_MainHudReference _returnvalue))
            (UserInterface|Viewport|AddtoViewport _output_get 0)
            (Variables|/Game/Core/Widgets/W_MainHud.W_MainHud_C|SetMatchTimeLength (Variables|Default|GetW_MainHudReference) 0.0)))
        (:Remote
          (goto _label))))))

(event EventCrossHairVisibility
  (params (IsCombact? :type Boolean))
  ;[0.15 0.15 0.15 0.5] Combat State Update
  ;;[0.15 0.15 0.15 0.5] Crosshair Visibilty Update
  (CallFunction|CrosshairHideOwningClient IsCombact?))

(event EventUpdateMiniMap
  (params (ReferenceToMaterialMiniMap :type Material%20Interface%20Object%20Reference))
  (CallFunction|UpdateMiniMaponOwningClient ReferenceToMaterialMiniMap))

(event EventUpdateGrenades
  (params (Number :type Integer))
  (Default|UpdateGrenadeNumber (Variables|Default|GetW_MainHudReference) Number))

(event EventUpdateLandMines
  (params (Number :type Integer))
  (CallFunction|HUDUpdateLandMines Number))

(event EventPopUpMessageAnnouncement
  (params (PopUpMessage :type Text))
  (CallFunction|HUDPlayMessagePopUp PopUpMessage))

(event EventSetUpPropWidget
  (params (IsProp? :type Boolean))
  ;[0.15 0.15 0.15 0.5] SetUp Widget Screen
  (Variables|Default|SetIs%20Prop? IsProp?)
  (CallFunction|SetProponClient IsProp?))

(event EventShowWinScreenWIdget
  (params (PropWon :type Boolean))
  ;[0.15 0.15 0.15 0.5] WinScreenWidget
  (CallFunction|ShowWinScreenonClient PropWon (Variables|Default|GetIs%20Prop?)))

(event EventCrosshairSpread
  (params (Velocity :type Vector :default "0, 0, 0"))
  ;[0.15 0.15 0.15 0.5] CrosshairSpread (the reason why we made it here, cuz our CONTROLLER HAS REFERENCE to HUD not OUR CHARACTER, however from our character we do need to COMMUNICATE VELOCITY
  ;;[0.15 0.15 0.15 0.5] Needed Step (CLIENT SPECIFIC)
  (CallFunction|SetupCrosshairSpreadonClient Velocity))

(event EventUpdateHealthWidget
  (params (Health :type Integer))
  ;[0.15 0.15 0.15 0.5] Health Update
  (CallFunction|UpdateHealthonClient Health))

(event EventSetMatchLengthandBeginCountdown
  (params (MatchTime :type Float%20%28double-precision%29))
  ;[0.15 0.15 0.15 0.5] Set 1)GameTimeLength 2)Trigger the Start Countdown
  (CallFunction|SetmatchLengthonClient MatchTime))

(event EventPlayCrosshairHit
  ;[0.15 0.15 0.15 0.5] CrossHair Hit
  (CallFunction|ShowCrosshaiirHitonClient))

(event EventWidgetAmmoCurrentInventoryGuninHand
  (params (Gun%20In%20Hand :type Integer) (Current%20Ammo :type Integer) (Inventory%20Ammo :type Integer))
  (CallFunction|HudUpdateGunHandAmmoMag Gun%20In%20Hand Current%20Ammo Inventory%20Ammo))

(event EventWidgetAmmoUpdate
  (params (Magzine%20Ammo :type Integer) (Inventory%20Ammo :type Integer))
  (CallFunction|HudUpdateAmmoMag Magzine%20Ammo Inventory%20Ammo))

(fn ConstructionScript)